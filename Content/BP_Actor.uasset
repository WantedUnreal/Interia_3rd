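; BP_Actor is a Blueprint scripting exercise that demonstrates basic variables, a function, branching and looping through printed messages.
; On BeginPlay, a Sequence prints MyName, reassigns it to a Korean string and prints it again, then prints the result of the Plus function on Number1 and Number2.
; It then prints which comparison branch the two numbers take and runs a short index loop with a completion message.
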(event `self.ReceiveBeginPlay`
  (`|ExecutionSequence`
    (:`then_0`
      (`KismetSystemLibrary.PrintString` (`self.MyName`)))
    (:`then_1`
      (set `self.MyName` "너무 교실이 더워요")
      (`KismetSystemLibrary.PrintString` (`self.MyName`)))
    (:`then_2`
      (bind _addvalue (`self.Plus` (`self.Number1`) (`self.Number2`)))
      (`KismetSystemLibrary.PrintString` (`KismetStringLibrary.Conv_IntToString` _addvalue)))
    (:`then_3`
      (if (> (`self.Number1`) (`self.Number2`))
        (`KismetSystemLibrary.PrintString` "Number1 이 Number2 보다 큽니다.")
        (else
          (`KismetSystemLibrary.PrintString` "Number1 이 Number2 보다 크지 않습니다."))))
    (:`then_4`
      (for _index (range 5)
        (`KismetSystemLibrary.PrintString` (`KismetStringLibrary.Conv_IntToString` _index)))
      (`KismetSystemLibrary.PrintString` "반복문 종료"))))

(event `self.ReceiveTick`
  (params (DeltaSeconds :type "Float (single-precision)")))

(fn `Plus`
  (params (Num1 :type Integer) (Num2 :type Integer))
  (returns (AddValue :type Integer))
  (return (+ Num1 Num2)))

(fn `UserConstructionScript`)